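; testCube is a test actor that tints its Cube component's "Color" material parameter pink at BeginPlay.
; Custom events TakeDamage and AddScore adjust Health and Score and print the new value.
; Disconnected practice snippets call those events, print PlayerName, test a win/lose score threshold and chain arithmetic on Score, but none of them runs.
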(event `self.ReceiveBeginPlay`
  (`MeshComponent.SetColorParameterValueOnMaterials` (`self.Cube`) "Color" (struct :`R` 0.963542 :`G` 0.612807 :`B` 0.921543 :`A` 1.0)))

(event `TakeDamage`
  (params (DamageAmount :type Integer))
  (bind _output_get (set `self.Health` (- (`self.Health`) DamageAmount)))
  (`KismetSystemLibrary.PrintString` (`KismetStringLibrary.Conv_IntToString` _output_get)))

(event `AddScore`
  (params (Amount :type Integer))
  (bind _output_get (set `self.Score` (+ (`self.Score`) Amount)))
  (`KismetSystemLibrary.PrintString` (`KismetStringLibrary.Conv_IntToString` _output_get)))

(event `self.ReceiveTick`
  (params (DeltaSeconds :type "Float (single-precision)")))

(fn `UserConstructionScript`)